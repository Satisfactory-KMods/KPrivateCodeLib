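; Creature spawner Blueprint whose own logic only visualizes its configured ranges; the event graph is empty.
; After the parent construction script, it checks MShowRanges and adds a sphere component for each MRanges entry, using that entry as the radius.
; The first entry is added through a separate sphere node from the remaining entries.
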(event EventBeginPlay)

(event Collision|EventActorBeginOverlap
  (params (OtherActor :type Actor%20Object%20Reference)))

(event EventTick
  (params (DeltaSeconds :type Float%20%28single-precision%29)))

(fn ConstructionScript
  (|CallParentFunction)
  (if (Variables|KMods|MapDisplay|GetmShowRanges)
    (for (_array_element _array_index) (Variables|KMods|MapDisplay|GetmRanges)
      (if (Math|Conversions|ToBoolean(Integer) _array_index)
        (bind _returnvalue (AddComponent|AddSphereComponent false))
        (Components|Sphere|SetSphereRadius _returnvalue _array_element true)
        (else
          (bind _returnvalue_2 (AddComponent|AddSphereComponent false))
          (Components|Sphere|SetSphereRadius _returnvalue_2 _array_element true))))))