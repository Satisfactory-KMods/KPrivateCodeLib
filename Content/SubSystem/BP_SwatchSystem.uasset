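; Subsystem that adds a config-gated custom swatch saver to the build gun's Customiser UI.
; Hooks BPW_Customiser Construct/Destruct to track the widget, then repeatedly searches on delayed Tick for the custom swatch slot to inject a save icon.
; Rebuilds saved-swatch buttons when that slot or swatch data changes, and shows or removes the editor in the color picker overlay.
; Paint gun validation is an empty stub with disconnected logic.
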(event Custom|CustomEvent_1
  (params (Object :type Object%20Object%20Reference))
  (Variables|Default|SetmCustomizer 0)
  (CallFunction|CloseEditor)
  (Variables|Default|SetmInit (Utilities|IsValid (Variables|Default|GetmCustomizer))))

(event Custom|mOnSwatchDataUpdated_Event_0
  (CallFunction|UpdateCustomDataSlots)
  (CallFunction|Todo?ValidatePainGunState))

(event Custom|CustomEvent_0
  (params (Object :type Object%20Object%20Reference))
  (bind _asbpw_customiser (Utilities|Casting|CastToBPW_Customiser Object))
  (Variables|Default|SetmCustomizer _asbpw_customiser)
  (Utilities|FlowControl|Delay 0.05)
  (CallFunction|CacheInfromations)
  (Variables|Default|SetmInit (Utilities|IsValid (Variables|Default|GetmCustomizer))))

(event EventBeginPlay
  (|CallParentFunction)
  (if (Class|KBFLConfigTools|GetBoolfromConfig "/KPrivateCodeLib/KPCL_Config.KPCL_Config_C" "UseCustomSwatchSaver")
    (Class|RuntimeBlueprintFunctionLibrary|BindonBPFunction "/Game/FactoryGame/Interface/UI/InGame/Customiser/BPW_Customiser.BPW_Customiser_C" (delegate Custom|CustomEvent_0) "Construct" false)
    (Class|RuntimeBlueprintFunctionLibrary|BindonBPFunction "/Game/FactoryGame/Interface/UI/InGame/Customiser/BPW_Customiser.BPW_Customiser_C" (delegate Custom|CustomEvent_1) "Destruct" false)
    (EventDispatchers|AssignMonSwatchDataUpdated (Class|KPCLSwatchSystem|Get) (delegate Custom|mOnSwatchDataUpdated_Event_0))))

(event EventTick
  (params (DeltaSeconds :type Float%20%28single-precision%29))
  (|CallParentFunction DeltaSeconds)
  (if (Class|KBFLConfigTools|GetBoolfromConfig "/KPrivateCodeLib/KPCL_Config.KPCL_Config_C" "UseCustomSwatchSaver")
    (Utilities|FlowControl|Delay 0.25)
    (Utilities|FlowControl|Sequence
      (:then_0
        (CallFunction|Todo?ValidatePainGunState))
      (:then_1
        (Utilities|IsValid (Variables|Default|GetmCustomizer)
          (:Is%20Valid
            (if (Variables|Default|GetmInit)
              (CallFunction|CacheInfromations))))))))

(fn ConstructionScript)

(fn UpdateCustomDataSlots
  (CallFunction|CloseEditor)
  (bind _arrayelement (Utilities|Array|ReverseforEachLoop (Class|PanelWidget|GetAllChildren (Variables|Default|GetmContainer)))
    (:LoopBody
      (bind _asbpw_kpcl_customiser_settings_button (Utilities|Casting|CastToBPW_KPCL_CustomiserSettingsButton _arrayelement))
      (Widget|RemovefromParent _asbpw_kpcl_customiser_settings_button))
    (:Completed
      (for (_array_element _array_index) (Class|KPCLSwatchSystem|GetCustomSwatchData (Class|KPCLSwatchSystem|Get))
        (bind _returnvalue (UserInterface|CreateWidget "/KPrivateCodeLib/SubSystem/BPW_KPCL_CustomiserSettingsButton.BPW_KPCL_CustomiserSettingsButton_C" 0 _array_element _array_index (Variables|Default|GetmCustomSlotButton)))
        (Class|WrapBox|AddChildtoWrapBox (Variables|Default|GetmContainer) _returnvalue)))))

(fn CacheInfromations
  (Variables|Default|SetmContainer 0)
  (Variables|Default|SetmCustomSlotButton 0)
  (Utilities|FlowControl|Sequence
    (:then_0
      (bind _array_element (Utilities|Array|ForEachLoopwithBreak (Class|PanelWidget|GetAllChildren (Variables|/Game/FactoryGame/Interface/UI/InGame/BuildMenu/Prototype/BPW_BuildMenu_Browser.BPW_BuildMenu_Browser_C|GetmSubCategoriesContainer (Variables|/Game/FactoryGame/Interface/UI/InGame/Customiser/BPW_Customiser.BPW_Customiser_C|GetBPW_BuildMenu_Browser (Variables|Default|GetmCustomizer)))) :!label _label)
        (:LoopBody
          (Utilities|IsValid (Variables|Default|GetmCustomSlotButton)
            (:Is%20Valid
              (goto _label Break))
            (:Is%20Not%20Valid
              (bind _aswidget_build_menu_sub_category_button (Utilities|Casting|CastToWidget_BuildMenu_SubCategoryButton _array_element))
              (bind _array_element_2 (Utilities|Array|ForEachLoopwithBreak (Class|PanelWidget|GetAllChildren (Variables|/Game/FactoryGame/Interface/UI/InGame/BuildMenu/Prototype/Widget_BuildMenu_SubCategoryButton.Widget_BuildMenu_SubCategoryButton_C|GetmBuildingsContainer _aswidget_build_menu_sub_category_button)) :!label _label_2)
                (:LoopBody
                  (bind _asbpw_customiser_settings_button (Utilities|Casting|CastToBPW_CustomiserSettingsButton _array_element_2))
                  (if (== (Variables|/Game/FactoryGame/Interface/UI/InGame/Customiser/BPW_CustomiserSettingsButton.BPW_CustomiserSettingsButton_C|GetmCustomiserDescriptor _asbpw_customiser_settings_button) (Variables|Default|GetmCustomSwatchSlot))
                    (Utilities|FlowControl|Sequence
                      (:then_0
                        (Variables|Default|SetmCustomSlotButton _asbpw_customiser_settings_button)
                        (Variables|Default|SetmContainer (Variables|/Game/FactoryGame/Interface/UI/InGame/BuildMenu/Prototype/Widget_BuildMenu_SubCategoryButton.Widget_BuildMenu_SubCategoryButton_C|GetmBuildingsContainer _aswidget_build_menu_sub_category_button)))
                      (:then_1
                        (LocalVariables|SetmLocal%20Exsists false)
                        (for _array_element_3 (Class|PanelWidget|GetAllChildren (Widget|GetParent (Variables|/Game/FactoryGame/Interface/UI/InGame/BuildMenu/Prototype/Widget_BuildMenu_SubCategoryButton.Widget_BuildMenu_SubCategoryButton_C|GetmNameBorder _aswidget_build_menu_sub_category_button)))
                          (Utilities|Casting|CastToBPW_KPCL_CustomiserSaveIcon _array_element_3)
                          (LocalVariables|SetmLocal%20Exsists true))
                        (if (not (LocalVariables|GetmLocal%20Exsists))
                          (bind _returnvalue (UserInterface|CreateWidget "/KPrivateCodeLib/SubSystem/BPW_KPCL_CustomiserSaveIcon.BPW_KPCL_CustomiserSaveIcon_C" 0 (Variables|Default|GetmCustomSlotButton)))
                          (Widget|Panel|AddChild (Widget|GetParent (Variables|/Game/FactoryGame/Interface/UI/InGame/BuildMenu/Prototype/Widget_BuildMenu_SubCategoryButton.Widget_BuildMenu_SubCategoryButton_C|GetmNameBorder _aswidget_build_menu_sub_category_button)) _returnvalue)))
                      (:then_2
                        (goto _label_2 Break)))))))))))
    (:then_1
      (Utilities|IsValid (Variables|Default|GetmCustomSlotButton)
        (:Is%20Valid
          (if (!= (Variables|Default|GetmCustomSlotButton) (Variables|Default|GetmLastCustomSlotButton))
            (Variables|Default|SetmLastCustomSlotButton (Variables|Default|GetmCustomSlotButton))
            (CallFunction|UpdateCustomDataSlots)))))))

(fn OpenEditor
  (params (Index :type Integer))
  (bind _mcustomizer (Variables|Default|GetmCustomizer))
  (Widget|SetVisibility (Variables|/Game/FactoryGame/Interface/UI/InGame/Customiser/BPW_Customiser.BPW_Customiser_C|GetmColorPickerBackground _mcustomizer) "Visible")
  (Class|BlueprintLoggingLibrary|LogDisplay "Open Editor!")
  (for _array_element (Class|PanelWidget|GetAllChildren (Variables|/Game/FactoryGame/Interface/UI/InGame/Customiser/BPW_Customiser.BPW_Customiser_C|GetmColorPickerSlot (Variables|Default|GetmCustomizer)))
    (bind _asbpw_kpcl_editor (Utilities|Casting|CastToBPW_KPCL_Editor _array_element))
    (Widget|SetVisibility _asbpw_kpcl_editor "Visible")
    (Default|SetupData _asbpw_kpcl_editor Index)
    (return))
  (bind _returnvalue (UserInterface|CreateWidget "/KPrivateCodeLib/SubSystem/BPW_KPCL_Editor.BPW_KPCL_Editor_C" 0 Index))
  (bind _returnvalue_2 (Class|Overlay|AddChildtoOverlay (Variables|/Game/FactoryGame/Interface/UI/InGame/Customiser/BPW_Customiser.BPW_Customiser_C|GetmColorPickerSlot _mcustomizer) _returnvalue))
  (Layout|GridSlot|SetHorizontalAlignment _returnvalue_2 "HAlign_Center")
  (Layout|GridSlot|SetVerticalAlignment _returnvalue_2 "VAlign_Center"))

(fn CloseEditor
  (bind _mcustomizer (Variables|Default|GetmCustomizer))
  (Utilities|IsValid _mcustomizer
    (:Is%20Valid
      (Widget|SetVisibility (Variables|/Game/FactoryGame/Interface/UI/InGame/Customiser/BPW_Customiser.BPW_Customiser_C|GetmColorPickerBackground _mcustomizer) "Collapsed")
      (for _array_element (Class|PanelWidget|GetAllChildren (Variables|/Game/FactoryGame/Interface/UI/InGame/Customiser/BPW_Customiser.BPW_Customiser_C|GetmColorPickerSlot _mcustomizer))
        (bind _asbpw_kpcl_editor (Utilities|Casting|CastToBPW_KPCL_Editor _array_element))
        (Widget|RemovefromParent _asbpw_kpcl_editor)))))

(fn Todo?ValidatePainGunState)