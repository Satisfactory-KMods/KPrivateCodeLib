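; Game world module that adds configured keybind widgets to the player HUD's shortcut grid.
; At Construction it binds to HUD widget creation, then creates, positions and initializes a widget for each MKeybindWidget entry.
; Entries alternate between two rows using the grid's child count, with a horizontal render offset for staggering.
; ShouldKeybindConstruct is a per-entry filter that currently always passes; ApplyEasyNodes separately forwards its nodes to EasyNodes.
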(event Custom|OnWidgetCreate
  (params (Widget :type User%20Widget%20Object%20Reference))
  (bind _aswidget_player_hud (Utilities|Casting|CastToWidget_PlayerHUD Widget))
  (Utilities|IsValid (Variables|/Game/FactoryGame/Character/Player/Widget_PlayerHUD.Widget_PlayerHUD_C|GetWidget_KeyShortcuts _aswidget_player_hud)
    (:Is%20Valid
      (for _array_element (Variables|KMods|Keybinding|GetmKeybindWidget)
        (bind _return (CallFunction|ShouldKeybindConstruct _array_element))
        (if _return
          (bind _returnvalue (UserInterface|CreateWidget (.mWidgetClass (Utilities|Struct|BreakKPCLKeybindInformation _array_element)) 0 _array_element))
          (Utilities|FlowControl|Sequence
            (:then_0
              (Class|Widget|SetRenderTranslation _returnvalue (select (not (== (Math|Integer|%(Integer) (Class|PanelWidget|GetChildrenCount (Variables|/Game/FactoryGame/Interface/UI/Widget_KeyShortcuts.Widget_KeyShortcuts_C|GetmGridBoxShortcuts (Variables|/Game/FactoryGame/Character/Player/Widget_PlayerHUD.Widget_PlayerHUD_C|GetWidget_KeyShortcuts _aswidget_player_hud))) 2) 0)) "(X=-26.000000,Y=0.000000)" "") :!label _label))
            (:then_1
              (bind _returnvalue_2 (Class|UniformGridPanel|AddChildtoUniformGrid (Variables|/Game/FactoryGame/Interface/UI/Widget_KeyShortcuts.Widget_KeyShortcuts_C|GetmGridBoxShortcuts (Variables|/Game/FactoryGame/Character/Player/Widget_PlayerHUD.Widget_PlayerHUD_C|GetWidget_KeyShortcuts _aswidget_player_hud)) _returnvalue (Math|Integer|SelectInt 1 0 (== (Math|Integer|%(Integer) (Class|PanelWidget|GetChildrenCount (Variables|/Game/FactoryGame/Interface/UI/Widget_KeyShortcuts.Widget_KeyShortcuts_C|GetmGridBoxShortcuts (Variables|/Game/FactoryGame/Character/Player/Widget_PlayerHUD.Widget_PlayerHUD_C|GetWidget_KeyShortcuts _aswidget_player_hud))) 2) 0)) (Math|Float|Truncate (* (Class|PanelWidget|GetChildrenCount (Variables|/Game/FactoryGame/Interface/UI/Widget_KeyShortcuts.Widget_KeyShortcuts_C|GetmGridBoxShortcuts (Variables|/Game/FactoryGame/Character/Player/Widget_PlayerHUD.Widget_PlayerHUD_C|GetWidget_KeyShortcuts _aswidget_player_hud))) 0.5))))
              (Layout|GridSlot|SetHorizontalAlignment _returnvalue_2 "HAlign_Left")
              (Layout|GridSlot|SetVerticalAlignment _returnvalue_2 "VAlign_Top")
              (goto _label))
            (:then_2
              (Default|Init _returnvalue))))))))

(event EventOnLifecycleEvent
  (params (Phase :type ELifecyclePhase%20Enum :default "CONSTRUCTION"))
  (switch Utilities|FlowControl|Switch|SwitchonELifecyclePhase Phase
    (:CONSTRUCTION
      (Class|KBFLWidgets|BindonWidget "/Game/FactoryGame/Character/Player/Widget_PlayerHUD.Widget_PlayerHUD_C" (delegate Custom|OnWidgetCreate)))))

(event EventApplyEasyNodes
  (params (Nodes :type Array%20of%20FG%20Research%20Tree%20Class%20References))
  (CallFunction|EasyNodes Nodes))

(fn ShouldKeybindConstruct
  (params (Information :type KPCL%20Keybind%20Information%20Structure))
  (return true))